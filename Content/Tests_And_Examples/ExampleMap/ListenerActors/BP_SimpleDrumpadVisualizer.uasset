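; BP_SimpleDrumpadVisualizer is an example listener actor that visualizes MIDI drum hits with animated blocks for kick, snare and hats.
; On BeginPlay it casts the three child actors to AnimatedBlock and maps each to a fixed note number.
; The listener component's MIDI events look up the block by note, making it ascend with the velocity on note-on and descend otherwise.
; Track option changes recolor all mapped blocks.
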(event OnMidiEvent(BP_ListenerComponentTest)
  (params (OutputName :type Name :default "None") (Output :type Meta%20Sound%20Output%20Structure%20%28by%20ref%29))
  (bind _returnvalue (Class|MidiEventInfoBlueprintLibrary|GetMidiEventInfo Output))
  (bind _returnvalue_2 (Class|MidiEventInfoBlueprintLibrary|GetVelocity _returnvalue))
  (bind _returnvalue_3 (Class|MidiEventInfoBlueprintLibrary|GetNoteNumber _returnvalue))
  (if (.ReturnValue (Utilities|Map|Find (Variables|Default|GetControlledBlocks) _returnvalue_3))
    (bind _returnvalue_4 (Class|MidiEventInfoBlueprintLibrary|IsNoteon _returnvalue))
    (if _returnvalue_4
      (Default|SetVelocity (.Value (Utilities|Map|Find (Variables|Default|GetControlledBlocks) _returnvalue_3)) (Math|Conversions|ToFloat(Integer) _returnvalue_2))
      (Default|Ascent (.Value (Utilities|Map|Find (Variables|Default|GetControlledBlocks) _returnvalue_3)))
      (else
        (Default|Descent (.Value (Utilities|Map|Find (Variables|Default|GetControlledBlocks) _returnvalue_3)))))))

(event OnTrackOptionsSet(BP_ListenerComponentTest)
  (params (TrackOptions :type Track%20Display%20Options%20Structure))
  (bind _values (Utilities|Map|Values (Variables|Default|GetControlledBlocks)))
  (for _array_element _values
    (Variables|/unDAW/Tests_And_Examples/ExampleMap/ListenerActors/Helpers/AnimatedBlock.AnimatedBlock_C|SetTrackColor _array_element (.trackColor (Utilities|Struct|BreakTrackDisplayOptions TrackOptions)))))

(event Custom|PopulateBlocks)

(event Custom|Cleanup
  (bind _outactors (Actor|GetAllActorsOfClasswithTag "/unDAW/Tests_And_Examples/ExampleMap/ListenerActors/Helpers/AnimatedBlock.AnimatedBlock_C" "MechanicalKeyCleanup"))
  (for _array_element _outactors
    (Actor|DestroyActor _array_element))
  (Utilities|Map|Clear (Variables|Default|GetControlledBlocks)))

(event EventBeginPlay
  (Utilities|Map|Clear (Variables|Default|GetControlledBlocks))
  (CallFunction|RegisterStaticMeshListener (Variables|Default|GetKick) 36)
  (CallFunction|RegisterStaticMeshListener (Variables|Default|GetSnare) 38)
  (CallFunction|RegisterStaticMeshListener (Variables|Default|GetHats) 46)
  (Variables|/unDAW/Tests_And_Examples/ExampleMap/ListenerActors/Helpers/AnimatedBlock.AnimatedBlock_C|SetMoveDistance (.Value (Utilities|Map|Find (Variables|Default|GetControlledBlocks) 38)) 5e+01))

(event Collision|EventActorBeginOverlap
  (params (OtherActor :type Actor%20Object%20Reference)))

(event EventTick
  (params (DeltaSeconds :type Float%20%28single-precision%29)))

(fn ConstructionScript)

(fn RegisterStaticMeshListener
  (params (self2 :type Child%20Actor%20Component%20Object%20Reference) (Key :type Integer))
  (bind _asanimated_block (Utilities|Casting|CastToAnimatedBlock (Variables|/Script/Engine.ChildActorComponent|GetChildActor self2)))
  (Utilities|Map|Add (Variables|Default|GetControlledBlocks) Key _asanimated_block)
  (return))