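; Calibration test actor that measures the average timing offset between MIDI metronome notes and user clicks.
; Four child AnimatedBlocks, mapped by note number, rise and fall on listener MIDI events and take the track's color.
; Note-ons store beat-quantized times from the audio-synced clock's bar and beat, assuming 75 BPM in 4/4.
; ReceiveClick subtracts these from the video-synced clock's smoothed audio position, printing and averaging the deltas.
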(event OnMidiEvent(BP_ListenerComponentTest)
  (params (OutputName :type Name :default "None") (Output :type Meta%20Sound%20Output%20Structure%20%28by%20ref%29))
  (bind _returnvalue (/ 6e+01 75.0))
  (bind _msactor (Variables|Default|GetMSActor))
  (bind _audiosyncedmidiclock (Variables|/Script/BKMusicCore.MusicScenePlayerActor|GetAudioSyncedMidiClock _msactor))
  (bind _returnvalue_2 (Class|MusicClockComponent|GetCurrentVideoRenderSongPos _audiosyncedmidiclock))
  (bind _returnvalue_3 (Math|Float|Floor (.beat (.timestamp _returnvalue_2))))
  (bind _returnvalue_4 (Math|Conversions|ToFloat(Integer) (.bar (.timestamp _returnvalue_2))))
  (bind _returnvalue_5 (Math|Conversions|ToFloat(Integer) _returnvalue_3))
  (bind _returnvalue_6 (|(BeatDuration*(((bar-1)*4)+beat)) _returnvalue_4 _returnvalue_5 _returnvalue))
  (bind _returnvalue_7 (Class|MidiEventInfoBlueprintLibrary|GetMidiEventInfo Output))
  (bind _returnvalue_8 (Class|MidiEventInfoBlueprintLibrary|GetVelocity _returnvalue_7))
  (bind _returnvalue_9 (Class|MidiEventInfoBlueprintLibrary|GetNoteNumber _returnvalue_7))
  (if (.ReturnValue (Utilities|Map|Find (Variables|Default|GetControlledBlocks) _returnvalue_9))
    (bind _returnvalue_10 (Class|MidiEventInfoBlueprintLibrary|IsNoteon _returnvalue_7))
    (if _returnvalue_10
      (Default|SetVelocity (.Value (Utilities|Map|Find (Variables|Default|GetControlledBlocks) _returnvalue_9)) (Math|Conversions|ToFloat(Integer) _returnvalue_8))
      (Default|Ascent (.Value (Utilities|Map|Find (Variables|Default|GetControlledBlocks) _returnvalue_9)))
      (Utilities|Map|Add (Variables|Default|GetMetronomeNoteTimes) _returnvalue_9 _returnvalue_6)
      (Development|PrintString (Utilities|String|ToString(Text) (Utilities|Text|FormatText "{note} happened at {time} 
CleanTime {CT}   
" _returnvalue_9 (.secondsfrombarone _returnvalue_2) _returnvalue_6)))
      (else
        (Default|Descent (.Value (Utilities|Map|Find (Variables|Default|GetControlledBlocks) _returnvalue_9)))))))

(event OnTrackOptionsSet(BP_ListenerComponentTest)
  (params (TrackOptions :type Track%20Display%20Options%20Structure))
  (bind _values (Utilities|Map|Values (Variables|Default|GetControlledBlocks)))
  (for _array_element _values
    (Variables|/unDAW/Tests_And_Examples/ExampleMap/ListenerActors/Helpers/AnimatedBlock.AnimatedBlock_C|SetTrackColor _array_element (.trackColor (Utilities|Struct|BreakTrackDisplayOptions TrackOptions)))))

(event Custom|PopulateBlocks)

(event Custom|Cleanup
  (bind _outactors (Actor|GetAllActorsOfClasswithTag "/unDAW/Tests_And_Examples/ExampleMap/ListenerActors/Helpers/AnimatedBlock.AnimatedBlock_C" "MechanicalKeyCleanup"))
  (for _array_element _outactors
    (Actor|DestroyActor _array_element))
  (Utilities|Map|Clear (Variables|Default|GetControlledBlocks)))

(event EventBeginPlay
  (Utilities|FlowControl|Sequence
    (:then_0
      (bind _returnvalue (Actor|GetActorOfClass "/Script/BKMusicCore.MusicScenePlayerActor"))
      (bind _output_get (Variables|Default|SetMSActor _returnvalue))
      (Variables|Default|SetVideo%20Synced%20Midi%20Clock (Variables|/Script/BKMusicCore.MusicScenePlayerActor|GetVideoSyncedMidiClock _output_get)))
    (:then_1
      (Utilities|Map|Clear (Variables|Default|GetControlledBlocks))
      (CallFunction|RegisterStaticMeshListener (Variables|Default|GetC) 84)
      (CallFunction|RegisterStaticMeshListener (Variables|Default|GetBb) 82)
      (CallFunction|RegisterStaticMeshListener (Variables|Default|GetA) 81)
      (CallFunction|RegisterStaticMeshListener (Variables|Default|GetG) 79))))

(event Collision|EventActorBeginOverlap
  (params (OtherActor :type Actor%20Object%20Reference)))

(event EventTick
  (params (DeltaSeconds :type Float%20%28single-precision%29)))

(fn ConstructionScript)

(fn RegisterStaticMeshListener
  (params (ChildActor :type Child%20Actor%20Component%20Object%20Reference) (Key :type Integer))
  (bind _asanimated_block (Utilities|Casting|CastToAnimatedBlock (Variables|/Script/Engine.ChildActorComponent|GetChildActor ChildActor)))
  (Utilities|Map|Add (Variables|Default|GetControlledBlocks) Key _asanimated_block)
  (return))

(fn ReceiveClick
  (params (Key :type Integer) (UserTime :type Float%20%28double-precision%29))
  (bind _metronomenotetimes (Variables|Default|GetMetronomeNoteTimes))
  (bind _video_synced_midi_clock (Variables|Default|GetVideo%20Synced%20Midi%20Clock))
  (bind _value (Utilities|Map|Find _metronomenotetimes Key))
  (bind _returnvalue (Class|MusicClockComponent|GetCurrentSmoothedAudioRenderSongPos _video_synced_midi_clock))
  (bind _returnvalue_2 (- (.secondsfrombarone _returnvalue) _value))
  (Utilities|Array|Add (Variables|Default|GetAccumulator) _returnvalue_2)
  (Development|PrintString (Utilities|String|ToString(Text) (Utilities|Text|FormatText "Note {note} : measured delta {delta}" Key _returnvalue_2)))
  (CallFunction|UpdateAverage))

(fn UpdateAverage
  (bind _accumulator (Variables|Default|GetAccumulator))
  (for _array_element _accumulator
    (LocalVariables|SetRunningValue (+ (LocalVariables|GetRunningValue) _array_element)))
  (Variables|Default|SetExperienced%20Average (/ (LocalVariables|GetRunningValue) (Utilities|Array|Length _accumulator))))