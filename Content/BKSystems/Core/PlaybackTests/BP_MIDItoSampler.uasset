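; Playback test actor that plays SFZ sampler notes through MetaSound audio components, driven by GameMode MIDI message dispatchers.
; Note-ons ask a Performer for an audio component stored per note, and note-offs trigger its MetaSound release.
; A placeholder sustain pedal pushes PedalState to stored components and prunes invalid ones.
; SFZ changes clear the Performer, whose creation is disconnected; direct MIDI-device binding is unused and CC is empty.
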(event Custom|MidiDeviceSelected
  (params (Device%20Name :type String))
  ;[1 1 1] update selected midi device
)

(event Custom|NoteOff
  (params (MIDIDeviceController :type MIDI%20Device%20Input%20Controller%20Object%20Reference) (Timestamp :type Integer) (Channel :type Integer) (Note :type Integer) (Velocity :type Integer))
  (bind _notetometamap (Variables|Default|GetnoteToMetaMAP))
  (bind (_value _returnvalue) (Utilities|Map|Find _notetometamap Note))
  (if _returnvalue
    (Utilities|IsValid _value
      (:Is%20Valid
        (Class|AudioParameterControllerInterface|SetTriggerParameter _value "MidiEngine.MidiNote.NoteOff")
        (if (not (Variables|Default|GetSustain%20Active))
          (Utilities|Map|Remove _notetometamap Note :!label _label)))
      (:Is%20Not%20Valid
        (goto _label)))))

(event Custom|NoteOn
  (params (MIDIDeviceController :type MIDI%20Device%20Input%20Controller%20Object%20Reference) (Timestamp :type Integer) (Channel :type Integer) (Note :type Integer) (Velocity :type Integer))
  (bind _audiocomponent (CallFunction|PerformNote (.Performer (Variables|Default|GetPerformer)) 0 Note Velocity))
  ;[1 1 1] Place Holder, should happen in performer code.
  (Effects|Components|ParticleSystem|SetBoolParameter _audiocomponent "FlyKick SFZ.Internals.PedalState" (Variables|Default|GetSustain%20Active))
  (Audio|Components|Audio|Play _audiocomponent 0.0)
  (Utilities|Map|Add (Variables|Default|GetnoteToMetaMAP) Note _audiocomponent))

(event Custom|midiCC
  (params (MIDIDeviceController :type MIDI%20Device%20Input%20Controller%20Object%20Reference) (Timestamp :type Integer) (Channel :type Integer) (Type :type Integer) (Value :type Integer)))

(event Custom|updateSFZmetasound)

(event Custom|SFZ%20Changed
  (params (New%20Debug%20SFZ%20Asset :type Object%20Object%20Reference))
  (Utilities|LoadAssetBlocking (Utilities|ResolveSoftReference New%20Debug%20SFZ%20Asset))
  (Variables|Default|SetSFZ 0 New%20Debug%20SFZ%20Asset)
  (Variables|Default|SetPerformer 0 (CallFunction|CreateSFZPerformerfromSampleBank New%20Debug%20SFZ%20Asset 0)))

(event Custom|Release_Complete
  (params (OutputName :type Name) (Output :type Meta%20Sound%20Output%20Structure%20%28by%20ref%29)))

(event Custom|Set%20Sustain%20Bool
  (params (Sustain%20Active :type Boolean))
  (bind _notetometamap (Variables|Default|GetnoteToMetaMAP))
  (bind _invalidacindexes (Variables|Default|GetInvalidACIndexes))
  ;[1 1 1] Hacky Pedal Demo
  (Variables|Default|SetSustain%20Active Sustain%20Active)
  (Utilities|IsValid (.Performer (Variables|Default|GetPerformer))
    (:Is%20Valid
      (Utilities|Array|Clear _invalidacindexes)
      (bind _keys (Utilities|Map|Keys _notetometamap))
      (for _array_element _keys
        (Utilities|IsValid (.Value (Utilities|Map|Find _notetometamap _array_element))
          (:Is%20Valid
            (Effects|Components|ParticleSystem|SetBoolParameter (.Value (Utilities|Map|Find _notetometamap _array_element)) "FlyKick SFZ.Internals.PedalState" (Variables|Default|GetSustain%20Active)))
          (:Is%20Not%20Valid
            (Utilities|Array|Add _invalidacindexes _array_element))))
      (for _array_element_2 _invalidacindexes
        (Utilities|Map|Remove _notetometamap _array_element_2)))))

(event EventBeginPlay
  (Utilities|FlowControl|Sequence
    (:then_0
      (bind _gm_base (Class|BPIGM|GetasGMBase(Message) (Game|GetGameMode)))
      (bind _output_get (Variables|Default|SetGM%20Base _gm_base))
      (EventDispatchers|BindEventtoDebugSFZInstrumentChanged _output_get (delegate Custom|SFZ%20Changed))
      (EventDispatchers|BindEventtoNoteonDispatcher (Variables|Default|GetGM%20Base) (EventDispatchers|CreateEvent :!event Custom|NoteOn))
      (EventDispatchers|BindEventtoMidiCCDispatcher (Variables|Default|GetGM%20Base) (EventDispatchers|CreateEvent :!event Custom|midiCC))
      (EventDispatchers|BindEventtoNoteOffDispatcher (Variables|Default|GetGM%20Base) (EventDispatchers|CreateEvent :!event Custom|NoteOff)))
    (:then_1
      (Utilities|LoadAssetBlocking (Utilities|ResolveSoftReference (stale Custom|SFZ%20Changed New%20Debug%20SFZ%20Asset)))
      (Variables|Default|SetSFZ 0 (stale Custom|SFZ%20Changed New%20Debug%20SFZ%20Asset))
      (Variables|Default|SetPerformer 0 (CallFunction|CreateSFZPerformerfromSampleBank (stale Custom|SFZ%20Changed New%20Debug%20SFZ%20Asset) 0)))))

(event Collision|EventActorBeginOverlap
  (params (OtherActor :type Actor%20Object%20Reference)))

(event EventTick
  (params (DeltaSeconds :type Float%20%28single-precision%29)))

(fn ConstructionScript)