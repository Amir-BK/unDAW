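; BP_MusicalActorTester is a test actor for spatialized music playback through the MusicManager.
; When a Pawn overlaps its Box, it spawns the Test_Action_Stinger2 patch attached to its root scene component with DiageticAttenuation.
; BeginPlay only prints a debug string.
; An unconnected branch that attaches the patch to the Master mixer input and prints the result never runs, and its callback event is empty.
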(event OnComponentBeginOverlap(Box)
  (params (OverlappedComponent :type Primitive%20Component%20Object%20Reference) (OtherActor :type Actor%20Object%20Reference) (OtherComp :type Primitive%20Component%20Object%20Reference) (OtherBodyIndex :type Integer) (bFromSweep :type Boolean) (SweepResult :type Hit%20Result%20Structure%20%28by%20ref%29))
  (Utilities|Casting|CastToPawn OtherActor)
  (Class|MusicScenePlayerActor|SpawnPatchAttached (Variables|Default|GetMusicManager) "/unDAW/Tests_And_Examples/Test_Action_Stinger2.Test_Action_Stinger2" (Variables|Default|GetDefaultSceneRoot) "None" "0, 0, 0" "0, 0, 0" "KeepRelativeOffset" false 1.0 1.0 0.0 "/unDAW/Tests_And_Examples/AudioBusses/DiageticAttenuation.DiageticAttenuation" 0))

(event Custom|CustomEvent
  (params (TriggerName :type Name)))

(event EventBeginPlay
  (Development|PrintString "What"))

(fn ConstructionScript)