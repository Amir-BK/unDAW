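; BP_unPatchActor is an example-map test actor whose events and construction script perform no work.
; Its event graph holds only disconnected experiments that never run.
; These touch on audio input device enumeration, audio capture creation and MetaSound source building with a custom patch node, alongside stray switch, print and loop nodes.
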(event Custom|CustomEvent_0
  (params (AvailableDevices :type Array%20of%20Audio%20Input%20Device%20Info%20Structures)))

(event EventBeginPlay)

(event Collision|EventActorBeginOverlap
  (params (OtherActor :type Actor%20Object%20Reference)))

(event EventTick
  (params (DeltaSeconds :type Float%20%28single-precision%29)))

(fn ConstructionScript)