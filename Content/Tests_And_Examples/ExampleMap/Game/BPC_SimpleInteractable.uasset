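; BPC_SimpleInteractable is an example scene component that an interactor can grab, highlight and release.
; Grab stores the interactor, sets the grabbed flag and returns itself, while Release clears both.
; While grabbed, Tick smoothly interpolates the component's world transform toward the interactor's grab location, without sweeping.
; The highlight event draws a short-lived debug sphere at the impact location.
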(event EventBeginPlay)

(event EventTick
  (params (DeltaSeconds :type Float%20%28single-precision%29))
  (if (Variables|Default|GetisGrabbed)
    (bind _transform (Default|GetGrabLocation (Variables|Default|GetInteractor)))
    (Transformation|SetWorldTransform (Class|KismetMathLibrary|TInterpto (Transformation|GetWorldTransform) _transform DeltaSeconds 0.9) false false)))

(event EventDrawInteractorHighlight
  (params (ImpactLocation :type Vector :default "0, 0, 0"))
  (Rendering|Debug|DrawDebugSphere ImpactLocation 15.0 12 "(R=1.000000,G=1.000000,B=1.000000,A=1.000000)" 0.1))

(event EventRelease
  (Variables|Default|SetisGrabbed false)
  (Variables|Default|SetInteractor 0))

(fn Grab
  (params (Interactor :type BPI%20Interactor%20Interface))
  (Variables|Default|SetInteractor Interactor)
  (Variables|Default|SetisGrabbed true)
  (return self))