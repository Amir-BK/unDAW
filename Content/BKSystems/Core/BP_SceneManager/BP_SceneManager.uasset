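; BP_SceneManager is a scene manager that connects playback transport to a SceneManagerTransportWidget hosted on its widget component.
; The construction script casts and caches the widget, and BeginPlay binds delegates in both directions.
; Widget clicks and seeks go out as transport and seek commands, with seeks guarded by a value comparison.
; Play state and seek target changes flow back to update the widget's display.
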(event Custom|3D%20widget%20clicked
  (params (NewCommand :type EBKTransportCommands%20Enum :default "Init"))
  (Class|BKMusicSceneManagerInterface|SendTransportCommand NewCommand))

(event Custom|CustomEvent
  (params (NewPlaystate :type EBKPlayState%20Enum :default "Preparing"))
  (Class|SceneManagerTransportWidget|SetTransportPlayState (Variables|Default|GetTransport%20Widget) NewPlaystate))

(event Custom|Set%203D%20Widget%20Transport%20Seek
  (params (NewSeekTarget :type Float%20%28single-precision%29))
  (Class|SceneManagerTransportWidget|SetTransportSeek (Variables|Default|GetTransport%20Widget) (stale Custom|TransportSeekDelegate_Event NewSeekTarget)))

(event Custom|Received%20Transport%20Seek%20From%203D%20widget
  (params (Value :type Float%20%28single-precision%29))
  (if (!= Value (Variables|Default|GetValue))
    (Variables|Default|SetValue Value)
    (Class|BKMusicSceneManagerInterface|SendSeekCommand Value)))

(event Custom|TransportSeekDelegate_Event
  (params (NewSeekTarget :type Float%20%28single-precision%29))
  (Class|SceneManagerTransportWidget|SetTransportSeek (Variables|Default|GetTransport%20Widget) NewSeekTarget))

(event Custom|Init%20Widget%20Binds)

(event EventBeginPlay
  (bind _transport_widget (Variables|Default|GetTransport%20Widget))
  (EventDispatchers|BindEventtoTransportCalled _transport_widget (delegate Custom|3D%20widget%20clicked))
  (EventDispatchers|BindEventtoPlaystateDelegate (delegate Custom|CustomEvent))
  (EventDispatchers|BindEventtoTransportSeekCommand _transport_widget (delegate Custom|Received%20Transport%20Seek%20From%203D%20widget))
  (EventDispatchers|BindEventtoTransportSeekDelegate (delegate Custom|Set%203D%20Widget%20Transport%20Seek)))

(event Collision|EventActorBeginOverlap
  (params (OtherActor :type Actor%20Object%20Reference)))

(event EventTick
  (params (DeltaSeconds :type Float%20%28single-precision%29)))

(event EventdSeekUpdate
  (params (InSeek :type Float%20%28single-precision%29))
  (Class|SceneManagerTransportWidget|SetTransportSeek (Variables|Default|GetTransport%20Widget) InSeek))

(fn ConstructionScript
  (bind _asscene_manager_transport_widget (Utilities|Casting|CastToSceneManagerTransportWidget (UserInterface|GetWidget (Variables|Default|GetWidget))))
  (Variables|Default|SetTransport%20Widget _asscene_manager_transport_widget)
  (CallFunction|InitWidgetBinds))