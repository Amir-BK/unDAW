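; Spectator pawn for the example map that highlights world objects under the camera and interacts with widgets.
; Each tick it traces 1500 units along the camera's forward vector against WorldDynamic and PhysicsBody objects, sending the hit component a DrawInteractorHighlight message with the impact point.
; Left mouse press and release drive the WidgetInteraction pointer key, and a press also reruns the highlight trace.
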(event EventBeginPlay)

(event Collision|EventActorBeginOverlap
  (params (OtherActor :type Actor%20Object%20Reference)))

(event EventTick
  (params (DeltaSeconds :type Float%20%28single-precision%29))
  (bind _returnvalue (Game|GetPlayerController 0))
  (bind _playercameramanager (Variables|/Script/Engine.PlayerController|GetPlayerCameraManager _returnvalue))
  (bind _returnvalue_2 (Camera|GetCameraLocation _playercameramanager))
  (bind (_outhit _returnvalue_3) (Collision|LineTraceForObjects _returnvalue_2 (+ (* (Math|Vector|GetForwardVector (Camera|GetCameraRotation _playercameramanager)) 1.5e+03) _returnvalue_2) (Utilities|Array|MakeArray "ObjectTypeQuery2" "ObjectTypeQuery4") false 0 "None"))
  (if _returnvalue_3
    (Class|BPISimpleInteractions|DrawInteractorHighlight(Message) (.HitComponent (Collision|BreakHitResult _outhit)) (.ImpactPoint (Collision|BreakHitResult _outhit)))))

(event Input|MouseEvents|LeftMouseButton
  (params (Key :type Key%20Structure :default "None"))
  (bind _returnvalue (Game|GetPlayerController 0))
  (bind _widgetinteraction (Variables|Default|GetWidgetInteraction))
  (bind _playercameramanager (Variables|/Script/Engine.PlayerController|GetPlayerCameraManager _returnvalue))
  (bind _returnvalue_2 (Camera|GetCameraLocation _playercameramanager))
  (:Pressed
    (Class|WidgetInteractionComponent|PressPointerKey _widgetinteraction Key)
    (bind (_outhit _returnvalue_3) (Collision|LineTraceForObjects _returnvalue_2 (+ (* (Math|Vector|GetForwardVector (Camera|GetCameraRotation _playercameramanager)) 1.5e+03) _returnvalue_2) (Utilities|Array|MakeArray "ObjectTypeQuery2" "ObjectTypeQuery4") false 0 "None"))
    (if _returnvalue_3
      (Class|BPISimpleInteractions|DrawInteractorHighlight(Message) (.HitComponent (Collision|BreakHitResult _outhit)) (.ImpactPoint (Collision|BreakHitResult _outhit)))))
  (:Released
    (Class|WidgetInteractionComponent|ReleasePointerKey _widgetinteraction Key)))

(fn ConstructionScript)