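; Builder helper that procedurally assembles a MetaSound source for multi-track MIDI playback through the MetaSound Builder API.
; InitSourceBuilder creates transport and click inputs, then runs the MIDI and track blocks.
; The MIDI block wires a manager node that outputs the MIDI stream and click audio.
; Each track channel-filters that stream into a Fusion sampler or custom patch, mixed with click through chained eight-channel stereo mixers, exposing per-track graph inputs.
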(fn InitSourceBuilder
  (params (OutputFormat :type EMetaSoundOutputAudioFormat%20Enum :default "Mono") (bIsOneShot :type Boolean) (BuilderName :type Name))
  (bind (_onplaynodeoutput _onfinishednodeinput _audiooutnodeinputs _returnvalue) (Class|MetaSoundBuilderSubsystem|CreateSourceBuilder (|MetaSoundBuilderSubsystem) BuilderName OutputFormat false)
    (:Succeeded
      (Utilities|FlowControl|Sequence
        (:then_0
          ;[1 1 1] Cache Default I/Os
          (Variables|BKAudio|MSBuilder|SetOn%20Finished%20Node%20Input _onfinishednodeinput)
          (Variables|BKAudio|MSBuilder|SetAudio%20Out%20Node%20Inputs _audiooutnodeinputs)
          (Variables|BKAudio|MSBuilder|SetOn%20Play%20Node%20Output _onplaynodeoutput)
          (Variables|BKAudio|MSBuilder|SetSource%20Builder _returnvalue))
        (:then_1
          (Class|MetaSoundBuilderBase|AddGraphInputNode (Variables|BKAudio|MSBuilder|GetSource%20Builder) "Play" "Trigger"
            (:Succeeded
              (bind _returnvalue_2 (Class|MetasoundFrontendLiteralBlueprintAccess|CreateBoolMetaSoundLiteral false))
              (Class|MetaSoundBuilderBase|AddGraphInputNode (Variables|BKAudio|MSBuilder|GetSource%20Builder) "Click" "bool" _returnvalue_2
                (:Succeeded
                  (Class|MetaSoundBuilderBase|AddGraphInputNode (Variables|BKAudio|MSBuilder|GetSource%20Builder) "Pause" "Trigger"
                    (:Succeeded
                      (Class|MetaSoundBuilderBase|AddGraphInputNode (Variables|BKAudio|MSBuilder|GetSource%20Builder) "Seek" "Trigger"
                        (:Succeeded
                          (Class|MetaSoundBuilderBase|AddGraphInputNode (Variables|BKAudio|MSBuilder|GetSource%20Builder) "SeekTarget" "Float"
                            (:Succeeded
                              (Class|MetaSoundBuilderBase|AddGraphInputNode (Variables|BKAudio|MSBuilder|GetSource%20Builder) "Continue" "Trigger"
                                (:Succeeded
                                  (Class|MetaSoundBuilderBase|AddGraphInputNode (Variables|BKAudio|MSBuilder|GetSource%20Builder) "Prepare" "Trigger"
                                    (:Succeeded
                                      (Class|MetaSoundBuilderBase|AddGraphInputNode (Variables|BKAudio|MSBuilder|GetSource%20Builder) "Stop" "Trigger"
                                        (:Succeeded
                                          (Class|MetaSoundBuilderBase|AddGraphOutputNode (Variables|BKAudio|MSBuilder|GetSource%20Builder) "MIDIStreamOut" "MIDIStream"))))))))))))))))))
        (:then_4
          (BKAudio|MSBuilder|InitMidiBlock)
          (BKAudio|MSBuilder|InitTracksBlock)
          (return (Variables|BKAudio|MSBuilder|GetSource%20Builder) true))))
    (:Failed
      (return 0 false))))

(fn InitMidiBlock
  (bind _source_builder (Variables|BKAudio|MSBuilder|GetSource%20Builder))
  (bind _source_builder_2 (Variables|BKAudio|MSBuilder|GetSource%20Builder))
  (bind _source_builder_3 (Variables|BKAudio|MSBuilder|GetSource%20Builder))
  (bind _source_builder_4 (Variables|BKAudio|MSBuilder|GetSource%20Builder))
  (Utilities|FlowControl|Sequence
    (:then_0
      ;[1 1 1] Set up Source inputs to Transport (Prepare on Play, we do not expose Midi file as input to Source for now)
      (Utilities|FlowControl|Sequence
        (:then_0
          (bind _returnvalue (Class|MetaSoundBuilderBase|AddNode (Variables|BKAudio|MSBuilder|GetSource%20Builder) (Variables|Default|GetNode%20Class))
            (:Succeeded
              (Utilities|Array|Add (Variables|Default|GetNodesArray) (Utilities|Struct|MakeST_NameToNode "Manager" _returnvalue))
              (bind _output_get (Variables|BKAudio|MSBuilder|Nodes|SetBKManagerNode _returnvalue))
              (Utilities|FlowControl|Sequence
                (:then_0
                  (bind _returnvalue_2 (Class|MetaSoundBuilderBase|FindNodeInputbyName _source_builder _output_get "Prepare")
                    (:Succeeded
                      (Class|MetaSoundBuilderBase|ConnectNodeInputtoGraphInput _source_builder "Prepare" _returnvalue_2
                        (:Succeeded
                          (bind _returnvalue_3 (Class|MetaSoundBuilderBase|FindNodeInputbyName _source_builder (Variables|BKAudio|MSBuilder|Nodes|GetBKManagerNode) "Pause")
                            (:Succeeded
                              (Class|MetaSoundBuilderBase|ConnectNodeInputtoGraphInput _source_builder "Pause" _returnvalue_3
                                (:Succeeded
                                  (bind _returnvalue_4 (Class|MetaSoundBuilderBase|FindNodeInputbyName _source_builder (Variables|BKAudio|MSBuilder|Nodes|GetBKManagerNode) "Seek Target")
                                    (:Succeeded
                                      (bind _returnvalue_5 (Class|MetaSoundBuilderBase|AddNodebyClassName _source_builder (Utilities|Struct|MakeMetasoundFrontendClassName "HarmonixNodes" "TimeMsToSeekTarget") 0)
                                        (:Succeeded
                                          (Utilities|Array|Add (Variables|Default|GetNodesArray) (Utilities|Struct|MakeST_NameToNode "TimeToMS" _returnvalue_5))
                                          (bind _returnvalue_6 (Class|MetaSoundBuilderBase|FindNodeInputbyName _source_builder _returnvalue_5 "Time (Ms)")
                                            (:Succeeded
                                              (Class|MetaSoundBuilderBase|ConnectNodeInputtoGraphInput _source_builder "SeekTarget" _returnvalue_6
                                                (:Succeeded
                                                  (bind _returnvalue_7 (Class|MetaSoundBuilderBase|FindNodeInputbyName _source_builder (Variables|BKAudio|MSBuilder|Nodes|GetBKManagerNode) "Trigger Seek")
                                                    (:Succeeded
                                                      (Variables|Default|SetTriggerSeek _returnvalue_7)
                                                      (bind _returnvalue_8 (Class|MetaSoundBuilderBase|FindNodeOutputbyName _source_builder _returnvalue_5 "Seek Target")
                                                        (:Succeeded
                                                          (Class|MetaSoundBuilderBase|ConnectNodes _source_builder _returnvalue_8 _returnvalue_4))))))))))))))))))))))
                (:then_1
                  (bind _returnvalue_9 (Class|MetaSoundBuilderBase|FindNodeInputbyName _source_builder _output_get "Play")
                    (:Succeeded
                      (Class|MetaSoundBuilderBase|ConnectNodeInputtoGraphInput _source_builder "Play" _returnvalue_9))))
                (:then_2
                  (bind _returnvalue_10 (Class|MetaSoundBuilderBase|FindNodeInputbyName _source_builder _output_get "Stop")
                    (:Succeeded
                      (Class|MetaSoundBuilderBase|ConnectNodeInputtoGraphInput _source_builder "Stop" _returnvalue_10))))
                (:then_3
                  (Class|MetaSoundBuilderBase|AddGraphInputNode _source_builder "MusicTimeStamp" "MusicTimestamp"
                    (:Succeeded
                      (Utilities|FlowControl|Sequence
                        (:then_0
                          (bind _returnvalue_11 (Class|MetaSoundBuilderBase|FindNodeInputbyName _source_builder_2 (Variables|BKAudio|MSBuilder|Nodes|GetBKManagerNode) "MusicTimeStamp")
                            (:Succeeded
                              (Class|MetaSoundBuilderBase|ConnectNodeInputtoGraphInput _source_builder_2 "MusicTimeStamp" _returnvalue_11
                                (:Succeeded
                                  (bind _output_get_2 (Variables|Default|SetMetaManagerNode (Variables|BKAudio|MSBuilder|Nodes|GetBKManagerNode)))
                                  (bind _returnvalue_12 (Class|MetaSoundBuilderBase|FindNodeInputbyName _source_builder_2 _output_get_2 "Trigger Seek")
                                    (:Succeeded
                                      (Class|MetaSoundBuilderBase|ConnectNodeInputtoGraphInput _source_builder_2 "Seek" _returnvalue_12))))))))))))))))))
    (:then_1
      (bind _returnvalue_13 (Class|MetasoundFrontendLiteralBlueprintAccess|CreateObjectMetaSoundLiteral (Variables|BKAudio|Midi|GetMidiFile)))
      (Class|MetaSoundBuilderBase|AddGraphInputNode _source_builder_3 "MidiFile" "MIDIAsset" _returnvalue_13))
    (:then_2
      (bind _output_get_3 (Variables|BKAudio|MSBuilder|Nodes|SetMidiPlayerNode (Variables|BKAudio|MSBuilder|Nodes|GetBKManagerNode)))
      (Utilities|FlowControl|Sequence
        (:then_0
          (bind _returnvalue_14 (Class|MetaSoundBuilderBase|FindNodeInputbyName _source_builder_3 (Variables|BKAudio|MSBuilder|Nodes|GetMidiPlayerNode) "MIDI File")
            (:Succeeded
              (Class|MetaSoundBuilderBase|ConnectNodeInputtoGraphInput _source_builder_4 "MidiFile" _returnvalue_14))))
        (:then_1
          (bind _returnvalue_15 (Class|MetaSoundBuilderBase|FindNodeInputbyName _source_builder_3 (Variables|BKAudio|MSBuilder|Nodes|GetMidiPlayerNode) "Transport")
            (:Succeeded
              (bind _returnvalue_16 (Class|MetaSoundBuilderBase|FindNodeOutputbyName _source_builder_3 (Variables|BKAudio|MSBuilder|Nodes|GetBKManagerNode) "Transport")
                (:Succeeded
                  (Class|MetaSoundBuilderBase|ConnectNodes _source_builder_4 _returnvalue_16 _returnvalue_15))))))
        (:then_2
          (bind _returnvalue_17 (Class|MetaSoundBuilderBase|FindNodeOutputbyName _source_builder_3 _output_get_3 "MIDI Stream")
            (:Succeeded
              (bind _output_get_4 (Variables|BKAudio|Midi|SetMidiStreamOutputHandle _returnvalue_17))
              (Class|MetaSoundBuilderBase|ConnectNodeOutputtoGraphOutput _source_builder_3 "MIDIStreamOut" _output_get_4))))
        (:then_3
          (bind _returnvalue_18 (Class|MetaSoundBuilderBase|FindNodeOutputbyName _source_builder_3 _output_get_3 "MIDI Clock")
            (:Succeeded
              (Class|MetaSoundBuilderBase|ConnectNodes _source_builder_3 _returnvalue_18 (LocalVariables|GetMidiClockTimeStampInput)))))))))

(fn InitTracksBlock
  (bind _metasoundfrontendclassname (Utilities|Struct|MakeMetasoundFrontendClassName "AudioMixer" "Audio Mixer (Stereo, 8)"))
  (bind _source_builder (Variables|BKAudio|MSBuilder|GetSource%20Builder))
  (bind _source_builder_2 (Variables|BKAudio|MSBuilder|GetSource%20Builder))
  (bind _midi_track_mappings (Variables|BKAudio|Midi|GetMidi%20Track%20Mappings))
  (bind _source_builder_3 (Variables|BKAudio|MSBuilder|GetSource%20Builder))
  (bind _source_builder_4 (Variables|BKAudio|MSBuilder|GetSource%20Builder))
  (bind _source_builder_5 (Variables|BKAudio|MSBuilder|GetSource%20Builder))
  (bind _source_builder_6 (Variables|BKAudio|MSBuilder|GetSource%20Builder))
  (Development|PrintString 0 (Utilities|GetDisplayName (Variables|Default|GetCurrentBuilder)))
  (Utilities|FlowControl|Sequence
    (:then_0
      ;[1 1 1] Assume Stereo For Now
      (bind _output_get (LocalVariables|SetNumChannels (+ (Utilities|Array|Length _midi_track_mappings) 2)))
      ;[1 1 1] Master Mixer, 8 channels are enough
      (bind _returnvalue (Class|MetaSoundBuilderBase|AddNodebyClassName _source_builder_4 _metasoundfrontendclassname)
        (:Succeeded
          (Utilities|Array|Add (Variables|Default|GetNodesArray) (Utilities|Struct|MakeST_NameToNode "Master" _returnvalue))
          (bind _output_get_2 (LocalVariables|SetMasterOutMixer _returnvalue))
          (Utilities|FlowControl|Sequence
            (:then_0
              (bind _returnvalue_2 (Class|MetaSoundBuilderBase|FindNodeOutputbyName _source_builder_4 _output_get_2 "Out L")
                (:Succeeded
                  (Class|MetaSoundBuilderBase|ConnectNodeOutputtoGraphOutput _source_builder_4 "UE.OutputFormat.Stereo.Audio:0" _returnvalue_2))))
            (:then_1
              (bind _returnvalue_3 (Class|MetaSoundBuilderBase|FindNodeOutputbyName _source_builder_4 _output_get_2 "Out R")
                (:Succeeded
                  (Class|MetaSoundBuilderBase|ConnectNodeOutputtoGraphOutput _source_builder_4 "UE.OutputFormat.Stereo.Audio:1" _returnvalue_3))))
            (:then_2
              (for _index (range 0 (/ _output_get 8))
                (bind _returnvalue_4 (Class|MetaSoundBuilderBase|AddNodebyClassName _source_builder_4 _metasoundfrontendclassname)
                  (:Succeeded
                    (Utilities|Array|Add (Variables|Default|GetNodesArray) (Utilities|Struct|MakeST_NameToNode "PreMaster" _returnvalue_4))
                    (Utilities|Array|Add (LocalVariables|GetMixerOutputNodeHandles) _returnvalue_4)
                    (Utilities|FlowControl|Sequence
                      (:then_0
                        (bind _returnvalue_5 (Class|MetaSoundBuilderBase|FindNodeInputbyName _source_builder_2 (LocalVariables|GetMasterOutMixer) (Utilities|String|StringToName (Utilities|String|ToString(Text) (Utilities|Text|FormatText "In {0} L" _index))))
                          (:Succeeded
                            (bind _returnvalue_6 (Class|MetaSoundBuilderBase|FindNodeOutputbyName _source_builder_2 _returnvalue_4 "Out L")
                              (:Succeeded
                                (Class|MetaSoundBuilderBase|ConnectNodes _source_builder_2 _returnvalue_6 _returnvalue_5))))))
                      (:then_1
                        (bind _returnvalue_7 (Class|MetaSoundBuilderBase|FindNodeInputbyName _source_builder_2 (LocalVariables|GetMasterOutMixer) (Utilities|String|StringToName (Utilities|String|ToString(Text) (Utilities|Text|FormatText "In {0} R" _index))))
                          (:Succeeded
                            (bind _returnvalue_8 (Class|MetaSoundBuilderBase|FindNodeOutputbyName _source_builder_2 _returnvalue_4 "Out R")
                              (:Succeeded
                                (Class|MetaSoundBuilderBase|ConnectNodes _source_builder_2 _returnvalue_8 _returnvalue_7)))))))))))))))
    (:then_1
      ;[1 1 1] For now we'll just add a fusion node, but this can easily be changed to accomodate metasound any metasound that accepts a MIDI stream and outputs audio
      (for (_array_element _array_index) _midi_track_mappings
        (LocalVariables|SetIndex _array_index)
        (LocalVariables|SetCurrentTrack _array_element)
        (switch Utilities|FlowControl|Switch|SwitchonETrackRendererMode (.RenderMode (Utilities|Struct|BreakTrackDisplayOptions _array_element))
          (:FusionPatch
            (bind _returnvalue_9 (Class|MetaSoundBuilderBase|AddNodebyClassName _source_builder (Utilities|Struct|MakeMetasoundFrontendClassName "HarmonixNodes" "FusionSamplerStereo") 0)
              (:Succeeded
                (LocalVariables|SetLocalPlayerNode _returnvalue_9))))
          (:CustomPatch
            (bind _returnvalue_10 (Class|MetaSoundBuilderBase|AddNode _source_builder (.MidiPatchClass (Utilities|Struct|BreakTrackDisplayOptions _array_element)))
              (:Succeeded
                (LocalVariables|SetLocalPlayerNode _returnvalue_10)))))
        (bind _returnvalue_11 (Class|MetaSoundBuilderBase|AddNodebyClassName _source_builder (Utilities|Struct|MakeMetasoundFrontendClassName "HarmonixNodes" "MidiChannelFilterNode") 0)
          (:Succeeded
            ;[1 1 1] Set up channel filter and midi stream
            (Utilities|FlowControl|Sequence
              (:then_0
                (bind _returnvalue_12 (Class|MetaSoundBuilderBase|FindNodeInputbyName _source_builder_6 _returnvalue_11 "MIDI Channel")
                  (:Succeeded
                    (bind _returnvalue_13 (Class|MetaSoundBuilderBase|FindNodeInputbyName _source_builder_6 _returnvalue_11 "MIDI Stream")
                      (:Succeeded
                        (bind _returnvalue_14 (Class|MetasoundFrontendLiteralBlueprintAccess|CreateIntMetaSoundLiteral (.ChannelIndexInParentMidi (Utilities|Struct|BreakTrackDisplayOptions (LocalVariables|GetCurrentTrack)))))
                        (bind _returnvalue_15 (Class|MetaSoundBuilderBase|AddGraphInputNode _source_builder_6 (Utilities|String|StringToName (Utilities|String|ToString(Text) (Utilities|Text|FormatText "Track{0}.MidiChannel" (LocalVariables|GetIndex)))) "int32" _returnvalue_14)
                          (:Succeeded
                            (Class|MetaSoundBuilderBase|ConnectNodes _source_builder_6 _returnvalue_15 _returnvalue_12
                              (:Succeeded
                                (Class|MetaSoundBuilderBase|ConnectNodes _source_builder_6 (Variables|BKAudio|Midi|GetMidiStreamOutputHandle) _returnvalue_13
                                  (:Succeeded
                                    (Utilities|FlowControl|Sequence
                                      (:then_0
                                        (bind _returnvalue_16 (Class|MetaSoundBuilderBase|FindNodeOutputbyName _source_builder_6 _returnvalue_11 "MIDI Stream")
                                          (:Succeeded
                                            (bind _returnvalue_17 (Class|MetaSoundBuilderBase|FindNodeInputbyName _source_builder_5 (LocalVariables|GetLocalPlayerNode) (Utilities|Select :Index (.RenderMode (Utilities|Struct|BreakTrackDisplayOptions (LocalVariables|GetCurrentTrack))) :FusionPatch "MIDI Stream" :CustomPatch "unDAW Instrument.MidiStream" :NoAudio "None"))
                                              (:Succeeded
                                                (Class|MetaSoundBuilderBase|ConnectNodes _source_builder_5 _returnvalue_16 _returnvalue_17))))))
                                      (:then_1
                                        (bind _returnvalue_18 (Class|MetasoundFrontendLiteralBlueprintAccess|CreateIntMetaSoundLiteral (.TrackIndexInParentMidi (Utilities|Struct|BreakTrackDisplayOptions (LocalVariables|GetCurrentTrack)))))
                                        (bind _returnvalue_19 (Class|MetaSoundBuilderBase|FindNodeInputbyName _source_builder_5 (LocalVariables|GetLocalPlayerNode) (Utilities|Select :Index (.RenderMode (Utilities|Struct|BreakTrackDisplayOptions (LocalVariables|GetCurrentTrack))) :FusionPatch "Track Number" :CustomPatch "unDAW Instrument.MidiTrack" :NoAudio "None"))
                                          (:Succeeded
                                            (bind _returnvalue_20 (Class|MetaSoundBuilderBase|AddGraphInputNode _source_builder_5 (Utilities|String|StringToName (Utilities|String|ToString(Text) (Utilities|Text|FormatText "Track{0}.TrackNumber" (LocalVariables|GetIndex)))) "int32" _returnvalue_18)
                                              (:Succeeded
                                                (Class|MetaSoundBuilderBase|ConnectNodes _source_builder_5 _returnvalue_20 _returnvalue_19
                                                  (:Succeeded
                                                    (switch Utilities|FlowControl|Switch|SwitchonETrackRendererMode (.RenderMode (Utilities|Struct|BreakTrackDisplayOptions (LocalVariables|GetCurrentTrack)))
                                                      (:FusionPatch
                                                        (bind _returnvalue_21 (Class|MetaSoundBuilderBase|FindNodeInputbyName _source_builder_5 (LocalVariables|GetLocalPlayerNode) "Patch")
                                                          (:Succeeded
                                                            (bind _returnvalue_22 (Class|MetasoundFrontendLiteralBlueprintAccess|CreateObjectMetaSoundLiteral (.fusionPatch (Utilities|Struct|BreakTrackDisplayOptions (LocalVariables|GetCurrentTrack)))))
                                                            (Class|MetaSoundBuilderBase|AddGraphInputNode _source_builder_5 (Utilities|String|StringToName (Utilities|String|ToString(Text) (Utilities|Text|FormatText "Track{0}.FusionPatch" (LocalVariables|GetIndex)))) "FusionPatchAsset" _returnvalue_22
                                                              (:Succeeded
                                                                (Class|MetaSoundBuilderBase|ConnectNodeInputtoGraphInput _source_builder_5 (Utilities|String|StringToName (Utilities|String|ToString(Text) (Utilities|Text|FormatText "Track{0}.FusionPatch" (LocalVariables|GetIndex)))) _returnvalue_21))))))))))))))
                                      (:then_2
                                        (bind _returnvalue_23 (Class|MetaSoundBuilderBase|FindNodeOutputbyName _source_builder_5 (LocalVariables|GetLocalPlayerNode) (Utilities|Select :Index (.RenderMode (Utilities|Struct|BreakTrackDisplayOptions (LocalVariables|GetCurrentTrack))) :FusionPatch "Audio Left" :CustomPatch "unDAW Instrument.Audio L" :NoAudio "None"))
                                          (:Succeeded
                                            (bind _returnvalue_24 (Class|MetaSoundBuilderBase|FindNodeOutputbyName _source_builder_5 (LocalVariables|GetLocalPlayerNode) (Utilities|Select :Index (.RenderMode (Utilities|Struct|BreakTrackDisplayOptions (LocalVariables|GetCurrentTrack))) :FusionPatch "Audio Right" :CustomPatch "unDAW Instrument.Audio R" :NoAudio "None"))
                                              (:Succeeded
                                                (bind _returnvalue_25 (Class|MetaSoundBuilderBase|FindNodeInputbyName _source_builder_5 (Utilities|Array|Get(acopy) (LocalVariables|GetMixerOutputNodeHandles) (/ (LocalVariables|GetIndex) 8)) (Utilities|String|StringToName (Utilities|String|ToString(Text) (Utilities|Text|FormatText "In {0} L" (Math|Integer|%(Integer) (LocalVariables|GetIndex) 8)))))
                                                  (:Succeeded
                                                    (Class|MetaSoundBuilderBase|ConnectNodes _source_builder_5 _returnvalue_23 _returnvalue_25
                                                      (:Succeeded
                                                        (bind _returnvalue_26 (Class|MetaSoundBuilderBase|FindNodeInputbyName _source_builder_5 (Utilities|Array|Get(acopy) (LocalVariables|GetMixerOutputNodeHandles) (/ (LocalVariables|GetIndex) 8)) (Utilities|String|StringToName (Utilities|String|ToString(Text) (Utilities|Text|FormatText "In {0} R" (Math|Integer|%(Integer) (LocalVariables|GetIndex) 8)))))
                                                          (:Succeeded
                                                            (Class|MetaSoundBuilderBase|ConnectNodes _source_builder_5 _returnvalue_24 _returnvalue_26
                                                              (:Succeeded
                                                                (bind _returnvalue_27 (Class|MetaSoundBuilderBase|FindNodeInputbyName _source_builder_5 (Utilities|Array|Get(acopy) (LocalVariables|GetMixerOutputNodeHandles) (/ (LocalVariables|GetIndex) 8)) (Utilities|String|StringToName (Utilities|String|ToString(Text) (Utilities|Text|FormatText "Gain {0}" (Math|Integer|%(Integer) (LocalVariables|GetIndex) 8)))))
                                                                  (:Succeeded
                                                                    (bind _returnvalue_28 (Class|MetasoundFrontendLiteralBlueprintAccess|CreateFloatMetaSoundLiteral (.TrackVolume (Utilities|Struct|BreakTrackDisplayOptions (LocalVariables|GetCurrentTrack)))))
                                                                    (bind _returnvalue_29 (Class|MetaSoundBuilderBase|AddGraphInputNode _source_builder_5 (Utilities|String|StringToName (Utilities|String|ToString(Text) (Utilities|Text|FormatText "Track{0}.Gain" (LocalVariables|GetIndex)))) "Float" _returnvalue_28)
                                                                      (:Succeeded
                                                                        (Class|MetaSoundBuilderBase|ConnectNodes _source_builder_5 _returnvalue_29 _returnvalue_27))))))))))))))))))))))))))))))))))
      ;[1 1 1] Click outputs setup
      (bind _returnvalue_30 (Class|MetaSoundBuilderBase|FindNodeOutputbyName _source_builder_3 (Variables|BKAudio|MSBuilder|Nodes|GetBKManagerNode) "Click Audio")
        (:Succeeded
          (bind _returnvalue_31 (Class|MetaSoundBuilderBase|FindNodeInputbyName _source_builder_3 (Utilities|Array|Get(acopy) (LocalVariables|GetMixerOutputNodeHandles) (/ (+ (LocalVariables|GetIndex) 1) 8)) (Utilities|String|StringToName (Utilities|String|ToString(Text) (Utilities|Text|FormatText "In {0} L" (Math|Integer|%(Integer) (+ (LocalVariables|GetIndex) 1) 8)))))
            (:Succeeded
              (bind _returnvalue_32 (Class|MetaSoundBuilderBase|FindNodeInputbyName _source_builder_3 (Utilities|Array|Get(acopy) (LocalVariables|GetMixerOutputNodeHandles) (/ (+ (LocalVariables|GetIndex) 1) 8)) (Utilities|String|StringToName (Utilities|String|ToString(Text) (Utilities|Text|FormatText "In {0} R" (Math|Integer|%(Integer) (+ (LocalVariables|GetIndex) 1) 8)))))
                (:Succeeded
                  (Class|MetaSoundBuilderBase|ConnectNodes _source_builder_3 _returnvalue_30 _returnvalue_31
                    (:Succeeded
                      (Class|MetaSoundBuilderBase|ConnectNodes _source_builder_3 _returnvalue_30 _returnvalue_32
                        (:Succeeded
                          (bind _returnvalue_33 (Class|MetaSoundBuilderBase|FindNodeInputbyName (Variables|BKAudio|MSBuilder|GetSource%20Builder) (Variables|BKAudio|MSBuilder|Nodes|GetBKManagerNode) "Click")
                            (:Succeeded
                              (Class|MetaSoundBuilderBase|ConnectNodeInputtoGraphInput _source_builder_3 "Click" _returnvalue_33))))))))))))))))