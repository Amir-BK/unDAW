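; GM_Base is a base game mode that manages the save object and MIDI input for a game using SFZ instruments.
; BeginPlay loads or creates the save, then binds to MIDI device and debug instrument selection events, which record choices in it.
; Selecting a device creates an input controller whose note on, note off and control change events are relayed through dispatchers.
; Tick feeds a Delay to autosave about every five seconds.
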(event Custom|MidiDeviceSelected
  (params (Device%20Name :type String))
  ;[1 1 1] update selected midi device
  (Variables|/BKAdaptiveMusic/BKSystems/Core/Save/BP_SaveGame.BP_SaveGame_C|SetMIDI%20Device%20Name (Variables|Default|GetSave%20Object) Device%20Name)
  (Utilities|FlowControl|Sequence
    (:then_0
      (Utilities|IsValid (Variables|Default|GetMIDI%20Device%20Controller)
        (:Is%20Valid
          (if (not (Utilities|Enum|Equal(Enum) (Variables|/Script/MIDIDevice.MIDIDeviceInputController|GetDeviceName (Variables|Default|GetMIDI%20Device%20Controller)) Device%20Name))
            (EventDispatchers|UnbindallEventsfromOnMIDINoteon (Variables|Default|GetMIDI%20Device%20Controller))))))
    (:then_1
      (bind _deviceid (Class|MIDIDeviceManager|GetMIDIInputDeviceIDbyName Device%20Name))
      (bind _returnvalue (Class|MIDIDeviceManager|CreateMIDIDeviceInputController _deviceid 256))
      (bind _output_get (Variables|Default|SetMIDI%20Device%20Controller _returnvalue))
      (Utilities|IsValid _output_get
        (:Is%20Valid
          (EventDispatchers|BindEventtoOnMIDINoteOff _output_get (EventDispatchers|CreateEvent :!event Custom|NoteOff))
          (EventDispatchers|BindEventtoOnMIDINoteon (Variables|Default|GetMIDI%20Device%20Controller) (EventDispatchers|CreateEvent :!event Custom|NoteOn))
          (EventDispatchers|BindEventtoOnMIDIControlChange _output_get (EventDispatchers|CreateEvent :!event Custom|midiCC)))))))

(event Custom|Debug%20SFZ%20Instrument%20Changed_Event
  (params (New%20Debug%20SFZ%20Asset :type Object%20Object%20Reference))
  (Variables|/BKAdaptiveMusic/BKSystems/Core/Save/BP_SaveGame.BP_SaveGame_C|SetSelected%20Instrument%20Name (Variables|Default|GetSave%20Object) (Utilities|GetDisplayName New%20Debug%20SFZ%20Asset)))

(event Custom|NoteOff
  (params (MIDIDeviceController :type MIDI%20Device%20Input%20Controller%20Object%20Reference) (Timestamp :type Integer) (Channel :type Integer) (Note :type Integer) (Velocity :type Integer))
  (Default|CallNoteOffDispatcher MIDIDeviceController Timestamp Channel Note Velocity))

(event Custom|midiCC
  (params (MIDIDeviceController :type MIDI%20Device%20Input%20Controller%20Object%20Reference) (Timestamp :type Integer) (Channel :type Integer) (Type :type Integer) (Value :type Integer))
  (Default|CallMidiCCDispatcher MIDIDeviceController Timestamp Channel Type Value))

(event Custom|NoteOn
  (params (MIDIDeviceController :type MIDI%20Device%20Input%20Controller%20Object%20Reference) (Timestamp :type Integer) (Channel :type Integer) (Note :type Integer) (Velocity :type Integer))
  (Default|CallNoteonDispatcher MIDIDeviceController Timestamp Channel Note Velocity))

(event EventBeginPlay
  (Utilities|FlowControl|Sequence
    (:then_0
      (bind _returnvalue (SaveGame|LoadGamefromSlot (Variables|Default|GetSlot%20Name)))
      (Utilities|IsValid _returnvalue
        (:Is%20Valid
          (bind _asbp_save_game (Utilities|Casting|CastToBP_SaveGame _returnvalue))
          (bind _output_get (Variables|Default|SetSave%20Object _asbp_save_game)))
        (:Is%20Not%20Valid
          (bind _returnvalue_2 (SaveGame|CreateSaveGameObject "/BKAdaptiveMusic/BKSystems/Core/Save/BP_SaveGame.BP_SaveGame_C"))
          (bind _returnvalue_3 (SaveGame|SaveGametoSlot _returnvalue_2 (Variables|Default|GetSlot%20Name)))
          (if _returnvalue_3
            (Variables|Default|SetSave%20Object _returnvalue_2)))))
    (:then_3
      (EventDispatchers|BindEventtoMidiInputSelected (delegate Custom|MidiDeviceSelected)))
    (:then_4
      (EventDispatchers|BindEventtoDebugSFZInstrumentChanged (delegate Custom|Debug%20SFZ%20Instrument%20Changed_Event)))))

(event EventTick
  (params (DeltaSeconds :type Float%20%28single-precision%29))
  (Utilities|FlowControl|Delay 5.0)
  (SaveGame|SaveGametoSlot (Variables|Default|GetSave%20Object) (Variables|Default|GetSlot%20Name)))

(event EventCallDebugSFZChanged
  (params (New%20SFZ%20Asset :type Object%20Object%20Reference))
  (Variables|/BKAdaptiveMusic/BKSystems/Core/Save/BP_SaveGame.BP_SaveGame_C|SetSFZ%20Asset%20Name (Variables|Default|GetSave%20Object) (Utilities|GetDisplayName New%20SFZ%20Asset))
  (Default|CallDebugSFZInstrumentChanged New%20SFZ%20Asset))

(fn ConstructionScript)

(fn GetasGMBase
  (return self))

(fn GetSaveObject
  (return (Variables|Default|GetSave%20Object)))