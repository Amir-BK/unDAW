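; Example cable connector component that snaps a simple interactable component into place when it comes within range.
; On BeginPlay it adds a scaled-up sphere component to its owner at its relative location and binds that sphere's begin overlap.
; When the overlapping component is a BPC_SimpleInteractable, it fires OnPinConnected, prints a debug string, attaches the interactable at its world transform and turns off its physics simulation.
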(event Custom|BeginOverlap
  (params (OverlappedComponent :type Primitive%20Component%20Object%20Reference) (OtherActor :type Actor%20Object%20Reference) (OtherComp :type Primitive%20Component%20Object%20Reference) (OtherBodyIndex :type Integer) (bFromSweep :type Boolean) (SweepResult :type Hit%20Result%20Structure%20%28by%20ref%29))
  (bind _asbpc_simple_interactable (Utilities|Casting|CastToBPC_SimpleInteractable OtherComp))
  (Default|CallOnPinConnected)
  (Development|PrintString "This Works")
  (Default|Attach _asbpc_simple_interactable (Transformation|GetWorldTransform))
  (Physics|SetSimulatePhysics _asbpc_simple_interactable false))

(event EventBeginPlay
  (bind _returnvalue (Game|AddComponentbyClass (Components|GetOwner) "/Script/Engine.SphereComponent" false (Math|Transform|MakeTransform (.location (Transformation|GetRelativeTransform)) "0, 0, 0" "5.000000,5.000000,5.000000")))
  (Collision|BindEventtoOnComponentBeginOverlap _returnvalue (delegate Custom|BeginOverlap)))

(event EventTick
  (params (DeltaSeconds :type Float%20%28single-precision%29)))