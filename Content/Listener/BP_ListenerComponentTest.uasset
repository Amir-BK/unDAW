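; A test listener component that relays one track's MIDI output from the audition MetaSound to event dispatchers.
; A tick after BeginPlay, it fetches display options for its TrackNumber from the SceneManager's session data and broadcasts OnTrackOptionsSet.
; It watches the MetaSound output named after the track on the audition AudioComponent via the MetaSound Output Subsystem, with changes intended to surface through OnMidiEvent.
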(event Custom|Midi%20Event
  (params (OutputName :type Name) (Output :type Meta%20Sound%20Output%20Structure%20%28by%20ref%29))
  (Default|CallOnMidiEvent OutputName Output))

(event EventBeginPlay
  (bind _scenemanager (Variables|Default|GetSceneManager))
  (bind _sessiondata (Variables|/Script/BKMusicCore.MusicScenePlayerActor|GetSessionData _scenemanager))
  (Utilities|FlowControl|DelayUntilNextTick)
  (bind _returnvalue (Class|DAWSequencerData|GetTracksDisplayOptions _sessiondata (Variables|unDAW|GetTrackNumber)))
  (bind _output_get (Variables|unDAW|SetTrackOptions _returnvalue))
  (MetaSoundOutput|WatchOutput (WorldSubsystems|GetMetaSoundOutputSubsystem) (Variables|/Script/BKMusicCore.DAWSequencerData|GetAuditionComponent _sessiondata) (Utilities|String|StringToName (.trackName (Utilities|Struct|BreakTrackDisplayOptions (Variables|unDAW|GetTrackOptions)))) (EventDispatchers|CreateEvent :!event Custom|Midi%20Event) "None" "None" :!class /Script/MetasoundEngine.MetaSoundOutputSubsystem)
  (Default|CallOnTrackOptionsSet _output_get))

(event EventTick
  (params (DeltaSeconds :type Float%20%28single-precision%29)))