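; Test actor that draws a DAW session's notes as a scrolling field of mesh instances.
; On BeginPlay it reads DAWListener's SessionData and creates one color-tinted instanced static mesh component per track.
; Notes are placed sideways by pitch and forward by start time scaled by UnitsPerSecond; the per-track drawn-note counter never advances.
; Tick moves the actor along world -X at a fixed speed, independent of UnitsPerSecond.
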(event EventBeginPlay
  (bind _output_get (Variables|Default|SetSession%20Data (Variables|/Script/BKMusicCore.MusicScenePlayerActor|GetSessionData (Variables|/Script/BKMusicCore.DAWListenerComponent|GetSceneManager (Variables|Default|GetDAWListener)))))
  (bind _keys (Utilities|Map|Keys (Variables|/Script/BKMusicCore.DAWSequencerData|GetLinkedNoteDataMap _output_get)))
  (for _array_element _keys
    (bind _returnvalue (Class|DAWSequencerData|GetTracksDisplayOptions _output_get _array_element))
    (bind _returnvalue_2 (Rendering|Material|CreateDynamicMaterialInstance "/Engine/BasicShapes/BasicShapeMaterial.BasicShapeMaterial" "None" "Transient" :!class /Script/Engine.KismetMaterialLibrary))
    (Rendering|Material|SetVectorParameterValue _returnvalue_2 "Color" (.trackColor (Utilities|Struct|BreakTrackDisplayOptions _returnvalue)) :!class /Script/Engine.MaterialInstanceDynamic)
    (bind _returnvalue_3 (AddComponent|AddInstancedStaticMeshComponent false))
    (Rendering|Material|SetMaterial _returnvalue_3 0 _returnvalue_2)
    (Utilities|Map|Add (Variables|Default|GetTrackToLastDrawnNote) _array_element 0)
    (Utilities|Map|Add (Variables|Default|GetTrackToMeshSpawnerMap) _array_element _returnvalue_3)
    (CallFunction|SpawnNotesinTrackandAdvanceCounter _array_element)))

(event Collision|EventActorBeginOverlap
  (params (OtherActor :type Actor%20Object%20Reference)))

(event EventTick
  (params (DeltaSeconds :type Float%20%28single-precision%29))
  (Transformation|AddActorWorldOffset (Math|Vector|MakeVector (* DeltaSeconds -1e+03) 0.0 0.0)))

(fn ConstructionScript)

(fn SpawnNotesinTrackandAdvanceCounter
  (params (TrackIndex :type Integer%20%28by%20ref%29))
  (bind _session_data (Variables|Default|GetSession%20Data))
  (bind _linkednotedatamap (Variables|/Script/BKMusicCore.DAWSequencerData|GetLinkedNoteDataMap _session_data))
  (bind _value (Utilities|Map|Find _linkednotedatamap TrackIndex))
  (bind _linkednotes (Utilities|Struct|BreakLinkedNotesTrack _value))
  (bind _index (Utilities|FlowControl|ForLoopwithBreak (.Value (Utilities|Map|Find (Variables|Default|GetTrackToLastDrawnNote) TrackIndex)) (Utilities|Array|Length _linkednotes))
    (:LoopBody
      (Development|PrintString (Utilities|String|ToString(Float) (.StartTime (Utilities|Struct|BreakLinkedMidiEvents (Utilities|Array|Get(acopy) _linkednotes _index)))))
      (bind _horizontaloffset (CallFunction|MapPitchHorizontally (Math|Conversions|ToInteger(Byte) (.pitch (Utilities|Struct|BreakLinkedMidiEvents (Utilities|Array|Get(acopy) _linkednotes _index))))))
      (Components|InstancedStaticMesh|AddInstance (.Value (Utilities|Map|Find (Variables|Default|GetTrackToMeshSpawnerMap) TrackIndex)) (Math|Conversions|ToTransform(Vector) (+ "" (* (Math|Vector|GetRightVector (Variables|Default|GetDefaultSceneRoot)) _horizontaloffset) (* (Math|Vector|GetForwardVector (Variables|Default|GetDefaultSceneRoot)) (* (.StartTime (Utilities|Struct|BreakLinkedMidiEvents (Utilities|Array|Get(acopy) _linkednotes _index))) (Variables|Default|GetUnitsPerSecond))))) false))))

(fn MapPitchHorizontally
  (params (Pitch :type Integer))
  (bind _out_range_a (Variables|Default|GetOut%20Range%20A))
  (return (Math|Float|MapRangeClamped (Math|Conversions|ToFloat(Integer) Pitch) 1.0 127.0 (* _out_range_a -1.0) _out_range_a)))